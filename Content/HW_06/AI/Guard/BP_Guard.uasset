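; AI guard character that draws and holsters a rifle for shooting, binds its health widget, and ragdolls on death before being destroyed.
; ModeShoot plays the equip montage forward when grounded to aim, or in reverse to holster.
; Montage notifies, filtered through Gate, FlipFlop and DoOnce nodes, move the rifle between spine and hand sockets, drive the DrawWeapon timeline and activate an ability.
; Death also unpossesses the AI controller.
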(event `self.Death`
  (bind _returnvalue (`AIBlueprintHelperLibrary.GetAIController` self))
  (`parent.Death`)
  (`self.Ragdoll`)
  (`/Engine/EditorBlueprintResources/StandardMacros.IsValid` _returnvalue
    (:`Is Valid`
      (`Controller.UnPossess` _returnvalue))
    (:`Is Not Valid`
      _))
  (`KismetSystemLibrary.Delay` 2.0)
  (`self.K2_DestroyActor`))

(event `self.ReceiveBeginPlay`
  (`parent.ReceiveBeginPlay`)
  (bind _aswbp_health (cast `/Game/HW_06/Widgets/WBP_Health` (`WidgetComponent.GetWidget` (`self.Widget`))))
  (set `/Game/HW_06/Widgets/WBP_Health.Owner` self _aswbp_health))

(event `ModeShoot`
  (params (Aim :type Boolean))
  (bind _rifle (`self.Rifle`))
  (bind _rifle_2 (`self.Rifle`))
  (if Aim
    (if (not (`NavMovementComponent.IsFalling` (`self.CharacterMovement`)))
      (`|ExecutionSequence`
        (:`then_0`
          (goto _label :!via `Open`))
        (:`then_1`
          (`|PlayMontage` (`self.Mesh`) "/Game/HW_06/Animations/MannyASP/Equip_Rifle_Montage.Equip_Rifle_Montage"
            (:`OnNotifyBegin`
              (`/Engine/EditorBlueprintResources/StandardMacros.Gate` true :!label _label
                (:`Exit`
                  (`|ExecutionSequence`
                    (:`then_0`
                      (`/Engine/EditorBlueprintResources/StandardMacros.FlipFlop`
                        (:`A`
                          (`SceneComponent.K2_AttachToComponent` _rifle_2 (`self.Mesh`) "hand_r" "KeepRelative" "KeepRelative" "KeepRelative" true)
                          (`SceneComponent.K2_SetRelativeTransform` _rifle_2 (`KismetMathLibrary.MakeTransform` (-11.590565 0.460342 4.436145) (struct :`Pitch` 3.986043 :`Yaw` 90.219046 :`Roll` -119.779275)) false false)
                          (`TimelineComponent.Play` (`self.DrawWeapon`)))
                        (:`B`
                          (`self.ActiveAbility` true "NewEnumerator6"))))
                    (:`then_1`
                      (goto _label_2 :!via `Reset`))))))))))
    (else
      (`|ExecutionSequence`
        (:`then_0`
          (goto _label :!via `Close`))
        (:`then_1`
          (`|PlayMontage` (`self.Mesh`) "/Game/HW_06/Animations/MannyASP/Equip_Rifle_Montage.Equip_Rifle_Montage" -1.0 1.13
            (:`then`
              (`self.ActiveAbility` false "NewEnumerator6"))
            (:`OnNotifyBegin`
              (`/Engine/EditorBlueprintResources/StandardMacros.DoOnce` true :!label _label_2
                (:`Completed`
                  (`TimelineComponent.Reverse` (`self.DrawWeapon`))
                  (`KismetSystemLibrary.Delay` 0.5)
                  (`SceneComponent.K2_AttachToComponent` _rifle (`self.Mesh`) "spine_03" "KeepRelative" "KeepRelative" "KeepRelative" true)
                  (`SceneComponent.K2_SetRelativeTransform` _rifle (`KismetMathLibrary.MakeTransform` (0.032848 -15.515569 3.087912) (struct :`Pitch` 8.57601 :`Yaw` -90.447712 :`Roll` 36.101486)) false false))))))))))

(fn `UserConstructionScript`)