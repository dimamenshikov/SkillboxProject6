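; Base character on the Gameplay Ability System, handling ability input, death and ragdoll.
; BeginPlay grants the Abilities map with key indices as input IDs, which ActiveAbility presses or releases by key.
; An attribute listener applies GE_Death once at zero or below, plays a sound, calls OnDeath and runs the empty Death hook.
; Non-lethal drops set PlayerDetected on an AIC_Guard's blackboard, while a separate Ragdoll event enables mesh physics.
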(event `self.ReceiveBeginPlay`
  (bind _abilities (`self.Abilities`))
  (bind _keys (`BlueprintMapLibrary.Map_Keys` _abilities))
  (for (_array_element _array_index) _keys
    (`AbilitySystemComponent.K2_GiveAbility` (`self.AbilitySystem`) (`BlueprintMapLibrary.Map_Find` _abilities _array_element) 0 _array_index))
  (bind (_asynctaskproxy _attribute _newvalue _oldvalue) (`AbilityAsync_WaitAttributeChanged.WaitForAttributeChanged` null (struct :`AttributeName` "Health" :`Attribute` "/Script/HW_06.HW_06AttributeSet:Health" :`AttributeOwner` "/Script/CoreUObject.Class'/Script/HW_06.HW_06AttributeSet'"))
    (:`Changed`
      (if (<= _newvalue 0.0)
        (`/Engine/EditorBlueprintResources/StandardMacros.DoOnce` false
          (:`Completed`
            (`AbilitySystemComponent.BP_ApplyGameplayEffectToSelf` :`self` (`self.AbilitySystem`) :`GameplayEffectClass` "/Game/HW_06/Blueprints/Abilities/Effects/GE_Death.GE_Death_C")
            (`GameplayStatics.PlaySoundAtLocation` "/Game/HW_06/Assets/Sound/A_Death.A_Death" (`self.K2_GetActorLocation`) (struct) 0.5 1.0 0.0 null null null null)
            (`self.OnDeath`)
            (`self.Death`)))
        (elif (< _newvalue _oldvalue)
          (bind _asaic_guard (cast `/Game/HW_06/AI/Guard/AIC_Guard` (`AIBlueprintHelperLibrary.GetAIController` self)))
          (`BlackboardComponent.SetValueAsBool` (`AIController.Blackboard` _asaic_guard) "PlayerDetected" true))))))

(event `Death`)

(event `Ragdoll`
  (bind _mesh (`self.Mesh`))
  (`PrimitiveComponent.SetCollisionEnabled` _mesh "PhysicsOnly")
  (`PrimitiveComponent.SetSimulatePhysics` _mesh true)
  (`PrimitiveComponent.SetCollisionEnabled` (`self.CapsuleComponent`) "NoCollision"))

(fn `ActiveAbility`
  (params (Activate :type Boolean) (Ability :type "/Game/HW_06/Blueprints/Abilities/E_Abilities Enum" :default "NewEnumerator0"))
  (bind _abilitysystem (`self.AbilitySystem`))
  (bind _keys (`BlueprintMapLibrary.Map_Keys` (`self.Abilities`)))
  (if Activate
    (bind _returnvalue (`KismetArrayLibrary.Array_Find` _keys Ability))
    (`AbilitySystemComponent.PressInputID` _abilitysystem _returnvalue)
    (else
      (`AbilitySystemComponent.ReleaseInputID` _abilitysystem _returnvalue))))

(fn `UserConstructionScript`)