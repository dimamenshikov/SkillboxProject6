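; Environment spawner actor that keeps two BP_Guard enemies alive inside a configurable box zone.
; On BeginPlay it caches world-space point locations from a referenced spline and hands them to each guard it spawns.
; Spawns use random XY in the box at the actor's Z, retrying recursively until a valid guard appears.
; Each guard's OnDeath event lowers the count and triggers a delayed respawn.
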(event `self.ReceiveBeginPlay`
  (for _index (range (`SplineComponent.GetNumberOfSplinePoints` (`/Game/HW_06/Blueprints/Environment/BP_PatrolRoute.Spline` (`self.Spline`))))
    (`KismetArrayLibrary.Array_Add` (`self.Points`) (`SplineComponent.GetLocationAtSplinePoint` (`/Game/HW_06/Blueprints/Environment/BP_PatrolRoute.Spline` (`self.Spline`)) _index "World")))
  (`self.SpawnEnem`))

(event `SpawnEnem`
  (bind (_returnvalue_x _returnvalue_y _returnvalue_z) (`KismetMathLibrary.BreakVector` (`self.K2_GetActorLocation`)))
  (bind _box (`self.Box`))
  (bind (_returnvalue_x_2 _returnvalue_y_2) (`KismetMathLibrary.BreakVector` (`KismetMathLibrary.RandomPointInBoundingBox` (`SceneComponent.K2_GetComponentLocation` _box) (`BoxComponent.GetScaledBoxExtent` _box))))
  (bind _returnvalue (`|SpawnActorFromClass` "/Game/HW_06/AI/Guard/BP_Guard.BP_Guard_C" (`KismetMathLibrary.MakeTransform` (`KismetMathLibrary.MakeVector` _returnvalue_x_2 _returnvalue_y_2 _returnvalue_z)) "AdjustIfPossibleButDontSpawnIfColliding" "MultiplyWithRoot" null null))
  (`/Engine/EditorBlueprintResources/StandardMacros.IsValid` _returnvalue
    (:`Is Valid`
      (set `/Game/HW_06/AI/Guard/BP_Guard.Points` (`self.Points`) _returnvalue)
      (`/Engine/EditorBlueprintResources/StandardMacros.IncrementInt` (`self.Count`)
        (:`  `
          (add `/Game/HW_06/Blueprints/Core/Character/BP_BaseCharacter.OnDeath` _returnvalue (delegate `DeathEnem`))
          (if (< (`self.Count`) 2)
            (`self.SpawnEnem`)))))
    (:`Is Not Valid`
      (`self.SpawnEnem`))))

(event `DeathEnem`
  (`/Engine/EditorBlueprintResources/StandardMacros.DecrementInt` (`self.Count`)
    (:`  `
      (`KismetSystemLibrary.Delay` 2.0)
      (`self.SpawnEnem`))))

(fn `UserConstructionScript`
  (bind _box (`self.Box`))
  (bind (_sizespawnzone_x _sizespawnzone_y _sizespawnzone_z) (`KismetMathLibrary.BreakVector` (`self.SizeSpawnZone`)))
  (`SceneComponent.K2_SetRelativeLocation` _box (`KismetMathLibrary.MakeVector` 0.0 0.0 _sizespawnzone_z) false false)
  (`BoxComponent.SetBoxExtent` _box (`self.SizeSpawnZone`) true))