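; BP_QuestManager gathers every BP_Quest actor in the level at BeginPlay and registers them in ascending order of their Number.
; It indexes quests in a temporary map, then repeatedly extracts the smallest key to fill the Quests map, a selection-sort approach.
; Each quest's OnComplete gets an event bound during that pass.
; The QuestComplete event and SortArray function are empty stubs.
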(event `self.ReceiveBeginPlay`
  (bind _tempmap (`self.TempMap`))
  (bind _outactors (`GameplayStatics.GetAllActorsOfClass` "/Game/HW_06/Blueprints/Environment/BP_Quest.BP_Quest_C"))
  (for _array_element _outactors
    (`BlueprintMapLibrary.Map_Add` (`self.TempMap`) (`/Game/HW_06/Blueprints/Environment/BP_Quest.Number` _array_element) _array_element))
  (bind _keys (`BlueprintMapLibrary.Map_Keys` _tempmap))
  (while (`KismetArrayLibrary.Array_IsNotEmpty` _keys)
    (bind (_indexofminvalue _minvalue) (`KismetMathLibrary.MinOfIntArray` _keys))
    (bind _value (`BlueprintMapLibrary.Map_Find` _tempmap _minvalue))
    (`BlueprintMapLibrary.Map_Add` (`self.Quests`) _minvalue _value)
    (add `/Game/HW_06/Blueprints/Environment/BP_Quest.OnComplete` _value (`|CreateDelegate` :!event `QuestComplete`))
    (`KismetArrayLibrary.Array_Remove` _keys _indexofminvalue)))

(event `QuestComplete`)

(fn `SortArray`
  (params (Array :type "Array of /Game/HW_06/Blueprints/Environment/BP_Quest Object Reference"))
  (locals (TempMap :type "Map of Integer to /Game/HW_06/Blueprints/Environment/BP_Quest Object Reference")))

(fn `UserConstructionScript`)